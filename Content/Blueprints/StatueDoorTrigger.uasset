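; StatueDoorTrigger is a trigger Blueprint that flashes a one-time spark effect when its trigger state becomes true.
; On BeginPlay it spawns a sparks effect actor at its own transform, hides the particles and clears their audio's sound.
; Tick polls GetTriggerState, which defers to the parent class, and a DoOnce briefly shows the sparks before hiding them again.
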(event `self.ReceiveBeginPlay`
  (bind _returnvalue (`|SpawnActorFromClass` "/Game/Blueprints/Blueprint_Effect_Sparks.Blueprint_Effect_Sparks_C" (`self.GetTransform`) "Undefined" "OverrideRootScale"))
  (set `self.SparkEffect` _returnvalue)
  (`SceneComponent.SetVisibility` (`/Game/Blueprints/Blueprint_Effect_Sparks.Sparks` (`self.SparkEffect`)) false false)
  (`AudioComponent.SetSound` (`/Game/Blueprints/Blueprint_Effect_Sparks.Sparks Audio` (`self.SparkEffect`)) null))

(event `self.ReceiveTick`
  (params (DeltaSeconds :type "Float (single-precision)"))
  (if (`self.GetTriggerState`)
    (`/Engine/EditorBlueprintResources/StandardMacros.DoOnce` false
      (:`Completed`
        (`SceneComponent.SetVisibility` (`/Game/Blueprints/Blueprint_Effect_Sparks.Sparks` (`self.SparkEffect`)) true false)
        (`KismetSystemLibrary.Delay` 0.05)
        (`SceneComponent.SetVisibility` (`/Game/Blueprints/Blueprint_Effect_Sparks.Sparks` (`self.SparkEffect`)) false false)))))

(fn `GetTriggerState`
  (returns (ReturnValue :type Boolean))
  (return (`parent.GetTriggerState`)))

(fn `UserConstructionScript`)