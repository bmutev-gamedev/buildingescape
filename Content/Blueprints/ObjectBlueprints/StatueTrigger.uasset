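; StatueTrigger is a trigger actor that gives a brief flash of sparks when its state becomes true.
; On BeginPlay it spawns a sparks effect actor at its own transform, hides the sparks and clears their audio sound.
; Tick polls GetState and, through a DoOnce with no reset, shows the sparks a single time before hiding them after a very short delay.
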(event `self.ReceiveBeginPlay`
  (bind _returnvalue (`|SpawnActorFromClass` "/Game/Blueprints/BP_Blueprint_Effect_Sparks.BP_Blueprint_Effect_Sparks_C" (`self.GetTransform`) "Undefined" "OverrideRootScale"))
  (set `self.SparkEffect` _returnvalue)
  (`SceneComponent.SetVisibility` (`/Game/Blueprints/BP_Blueprint_Effect_Sparks.Sparks` (`self.SparkEffect`)) false false)
  (`AudioComponent.SetSound` (`/Game/Blueprints/BP_Blueprint_Effect_Sparks.Sparks Audio` (`self.SparkEffect`)) null))

(event `self.ReceiveTick`
  (params (DeltaSeconds :type "Float (single-precision)"))
  (if (`self.GetState`)
    (`/Engine/EditorBlueprintResources/StandardMacros.DoOnce` false
      (:`Completed`
        (`SceneComponent.SetVisibility` (`/Game/Blueprints/BP_Blueprint_Effect_Sparks.Sparks` (`self.SparkEffect`)) true false)
        (`KismetSystemLibrary.Delay` 0.05)
        (`SceneComponent.SetVisibility` (`/Game/Blueprints/BP_Blueprint_Effect_Sparks.Sparks` (`self.SparkEffect`)) false false)))))

(fn `UserConstructionScript`)