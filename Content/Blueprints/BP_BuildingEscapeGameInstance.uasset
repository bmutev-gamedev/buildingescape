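; Game instance for Building Escape that applies and persists the graphics quality preset.
; InitSettings loads the preset from a SaveSettings save game if one exists; otherwise it applies the passed Quality and saves it to a new slot.
; Four preset functions (Low, Medium, High, Ultra for "PC Master Race Machine") set resolution and scalability levels through console commands.
; An existing save always overrides the passed Quality and is never rewritten here.
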(event `InitSettings`
  (params (Quality :type String))
  ;[1 1 1] Load graphic settings if a settings file exist
  (bind _returnvalue (`GameplayStatics.DoesSaveGameExist` (`self.Filename_Graphics`)))
  (if _returnvalue
    (bind _graphicsquality (`self.LoadGraphicsSettings`))
    (switch `string` _graphicsquality
      (:`Low`
        (`self.Low`))
      (:`Medium`
        (`self.Medium`))
      (:`High`
        (`self.High`))
      (:`PCMasterRaceMachine`
        (`self.Ultra`)))
    (else
      ;[1 1 1] If there is no GraphicsSettings file create one and save the settings
      (switch `string` Quality
        (:`Low`
          (set `self.SettingsQuality` "NewEnumerator0")
          (`self.Low`))
        (:`Medium`
          (set `self.SettingsQuality` "NewEnumerator1")
          (`self.Medium`))
        (:`High`
          (set `self.SettingsQuality` "NewEnumerator2")
          (`self.High`))
        (:`PCMasterRaceMachine`
          (set `self.SettingsQuality` "NewEnumerator3")
          (`self.Ultra`)))
      (`self.SaveGraphicSettings`))))