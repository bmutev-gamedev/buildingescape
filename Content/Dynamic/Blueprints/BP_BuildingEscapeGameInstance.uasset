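; Game instance for Building Escape that applies and persists graphics quality presets.
; InitSettings switches on a quality choice to Low, Medium, High or Ultra functions, each running console commands for resolution, shadows, textures, effects, post-processing, anti-aliasing and resolution scale.
; SaveGraphicSettings writes the chosen preset to a SaveSettings slot, and LoadGraphicsSettings reads it back as a string.
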(event `InitSettings`
  (params (Quality :type String))
  (switch `string` Quality
    (:`Low`
      (`self.Low`))
    (:`Medium`
      (`self.Medium`))
    (:`High`
      (`self.High`))
    (:`PCMasterRaceMachine`
      (`self.Ultra`))))